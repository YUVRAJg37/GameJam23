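; Player aircraft that handles mouse steering input, missile attacks, damage effects and crash death, with an on-screen widget for status messages.
; Missiles fire from a socket only when homing targets exist, then wait out a cooldown.
; Sacrifice adjusts fire rate to regain health, bounded by max health and minimum fire rate.
; Damage at low health spawns fire, while any hit triggers explosion, camera shake, destruction and the death screen.
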(event EventBeginPlay
  ;[1 1 0] Create and Set Widgets Hidden
  (bind _returnvalue (UserInterface|CreateWidget "/Game/Blueprints/WBP_Aircraft.WBP_Aircraft_C"))
  (bind _output_get (Variables|Default|SetAircraft%20Widget _returnvalue))
  (UserInterface|Viewport|AddtoViewport _output_get 0)
  (Widget|SetVisibility (Variables|/Game/Blueprints/WBP_Aircraft.WBP_Aircraft_C|GetSacrifice (Variables|Default|GetAircraft%20Widget)) "Hidden")
  (Widget|SetVisibility (Variables|/Game/Blueprints/WBP_Aircraft.WBP_Aircraft_C|GetHealthFull (Variables|Default|GetAircraft%20Widget)) "Hidden")
  (Widget|SetVisibility (Variables|/Game/Blueprints/WBP_Aircraft.WBP_Aircraft_C|GetAbortLaunch (Variables|Default|GetAircraft%20Widget)) "Hidden")
  (Widget|SetVisibility (Variables|/Game/Blueprints/WBP_Aircraft.WBP_Aircraft_C|GetMaxSacrifice (Variables|Default|GetAircraft%20Widget)) "Hidden"))

(event Collision|EventHit
  (params (MyComp :type Primitive%20Component%20Object%20Reference) (Other :type Actor%20Object%20Reference) (OtherComp :type Primitive%20Component%20Object%20Reference) (bSelfMoved :type Boolean) (HitLocation :type Vector :default "0, 0, 0") (HitNormal :type Vector :default "0, 0, 0") (NormalImpulse :type Vector :default "0, 0, 0") (Hit :type Hit%20Result%20Structure%20%28by%20ref%29))
  ;[0 1 1] Explode Aircraft
  (if (not (Variables|Default|GetDestroying))
    (Variables|Default|SetDestroying true)
    (CallFunction|ExplodeAircraft)
    (Class|LegacyCameraShake|StartLegacyCameraShake (Game|GetPlayerCameraManager 0) "/Game/Blueprints/BP_CameraShake.BP_CameraShake_C" 1.0 "CameraLocal" "0, 0, 0")
    (Utilities|FlowControl|Delay 1.25)
    (Widget|SetVisibility (Variables|Default|GetAircraft%20Widget) "Hidden")
    (Actor|DestroyActor)
    (bind _returnvalue (UserInterface|CreateWidget "/Game/Widgets/WBP_DeathScreen.WBP_DeathScreen_C"))
    (UserInterface|Viewport|AddtoViewport _returnvalue 0)
    (Variables|/Script/Engine.PlayerController|SetbShowMouseCursor (Game|GetPlayerController 0) true)))

(event Game|Damage|EventAnyDamage
  (params (Damage :type Float%20%28single-precision%29) (DamageType :type Damage%20Type%20Object%20Reference) (InstigatedBy :type Controller%20Object%20Reference) (DamageCauser :type Actor%20Object%20Reference))
  (bind _planemesh (Variables|Default|GetPlaneMesh))
  (bind _returnvalue (Transformation|GetSocketTransform _planemesh "Smoke" "RTS_World"))
  ;[0 0.5 0] Fire Effects
  (if (<= (Variables|Default|GetHealth) 4e+01)
    (Effects|SpawnEmitteratLocation "/Game/StarterContent/Particles/P_Fire.P_Fire" (.location _returnvalue) (.rotation _returnvalue) (.scale _returnvalue) false)))

(event Input|ActionEvents|InputActionSacrifice
  (params (Key :type Key%20Structure :default "None"))
  (bind _aircraft_widget (Variables|Default|GetAircraft%20Widget))
  (bind _aircraft_widget_2 (Variables|Default|GetAircraft%20Widget))
  (bind _aircraft_widget_3 (Variables|Default|GetAircraft%20Widget))
  (bind _healthfull (Variables|/Game/Blueprints/WBP_Aircraft.WBP_Aircraft_C|GetHealthFull _aircraft_widget_2))
  (bind _maxsacrifice (Variables|/Game/Blueprints/WBP_Aircraft.WBP_Aircraft_C|GetMaxSacrifice _aircraft_widget))
  (bind _sacrifice (Variables|/Game/Blueprints/WBP_Aircraft.WBP_Aircraft_C|GetSacrifice _aircraft_widget_3))
  ;[0 0 0.5 0.5] Sacrifice
  (:Pressed
    (if (< (Variables|Default|GetHealth) (Variables|Default|GetMaxHealth))
      (if (> (Variables|Default|GetFireRate) (Variables|Default|GetMinFireRate))
        (Variables|Default|SetHealth (+ (Variables|Default|GetHealth) (Variables|Default|GetHealthIncrement)))
        (Variables|Default|SetFireRate (+ (Variables|Default|GetFireRate) (Variables|Default|GetFireRateIncrement)))
        (Widget|SetVisibility _sacrifice "Visible")
        (Utilities|FlowControl|Delay 2.0)
        (Widget|SetVisibility _sacrifice "Hidden")
        (else
          (Widget|SetVisibility (Variables|/Game/Blueprints/WBP_Aircraft.WBP_Aircraft_C|GetSacrifice _aircraft_widget) "Hidden")
          (Widget|SetVisibility _maxsacrifice "Visible")
          (Utilities|FlowControl|Delay 2.0)
          (Widget|SetVisibility _maxsacrifice "Hidden")))
      (else
        (Widget|SetVisibility (Variables|/Game/Blueprints/WBP_Aircraft.WBP_Aircraft_C|GetSacrifice _aircraft_widget_2) "Hidden")
        (Widget|SetVisibility _healthfull "Visible")
        (Utilities|FlowControl|Delay 2.0)
        (Widget|SetVisibility _healthfull "Hidden")))))

(event Input|ActionEvents|InputActionLaunchMissile
  (params (Key :type Key%20Structure :default "None"))
  (bind _aircraft_widget (Variables|Default|GetAircraft%20Widget))
  (bind _abortlaunch (Variables|/Game/Blueprints/WBP_Aircraft.WBP_Aircraft_C|GetAbortLaunch _aircraft_widget))
  ;[1 1 1] Launch Missile
  (:Pressed
    (bind _outactors (Actor|GetAllActorsOfClass "/Game/Blueprints/BP_HomingTarget.BP_HomingTarget_C"))
    (if (> (Utilities|Array|Length _outactors) 0)
      (if (Variables|Default|GetMissileAmmo)
        (bind _returnvalue (Game|SpawnActorfromClass "/Game/Blueprints/BP_Missile.BP_Missile_C" (Transformation|GetSocketTransform (Variables|Default|GetPlaneMesh) "MachineGunFire" "RTS_World") "Undefined" 0 0))
        (Variables|Default|SetProjectile _returnvalue)
        (Audio|PlaySound2D "/Game/MilitaryWeapDark/Sound/GrenadeLauncher/GrenadeLauncherB_Fire_Cue.GrenadeLauncherB_Fire_Cue" 1.0 1.0 0.0 0 0)
        (Variables|Default|SetMissileAmmo false)
        (Utilities|FlowControl|Delay (Variables|Default|GetMissile%20Cooldown))
        (Variables|Default|SetMissileAmmo true))
      (else
        (Widget|SetVisibility _abortlaunch "Visible")
        (Utilities|FlowControl|Delay 2.0)
        (Widget|SetVisibility _abortlaunch "Hidden")))))

(event Input|MouseEvents|MouseY
  (params (AxisValue :type Float%20%28single-precision%29))
  ;[1 0 0] Plane Roll
  (Class|Aircraft|MouseYInput AxisValue))

(event Input|MouseEvents|MouseX
  (params (AxisValue :type Float%20%28single-precision%29))
  ;[1 0 0] Plane Roll
  (Class|Aircraft|MouseXInput AxisValue))

(fn ConstructionScript)

(fn ExplodeAircraft
  (bind _returnvalue (Transformation|GetActorTransform))
  (Effects|SpawnEmitteratLocation "/Game/MilitaryWeapDark/FX/P_Grenade_Explosion_01.P_Grenade_Explosion_01" (.location _returnvalue) (.rotation _returnvalue) (.scale _returnvalue))
  (Audio|PlaySound2D "/Game/MilitaryWeapDark/Sound/GrenadeLauncher/GrenadeLauncher_Explosion_Cue.GrenadeLauncher_Explosion_Cue" 1.0 1.0 0.0 0 0)
  (Development|SetHiddeninGame (Variables|Default|GetPlaneMesh) true false))

(fn OnRepPlaneHealth)