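; BP_Missile is a homing missile that seeks BP_Turret actors and destroys them on overlap.
; After LockOnTime, a BeginPlay loop re-runs Lockon every 0.1 seconds, feeding FindHomingTarget's result into the projectile's homing component.
; FindHomingTarget tracks the smallest distance but assigns the target before comparing, so it returns the last valid turret.
; Turret overlap plays explosion sound and particles, shakes the camera and destroys both actors.
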(event OnComponentBeginOverlap(CollisionSphere)
  (params (OverlappedComponent :type Primitive%20Component%20Object%20Reference) (OtherActor :type Actor%20Object%20Reference) (OtherComp :type Primitive%20Component%20Object%20Reference) (OtherBodyIndex :type Integer) (bFromSweep :type Boolean) (SweepResult :type Hit%20Result%20Structure%20%28by%20ref%29))
  ;[1 1 0] Explode
  (bind _asbp_turret (Utilities|Casting|CastToBP_Turret OtherActor))
  (Audio|PlaySound2D "/Game/MilitaryWeapDark/Sound/GrenadeLauncher/GrenadeLauncher_Explosion_Cue.GrenadeLauncher_Explosion_Cue" 1.0 1.0 0.0 0 0)
  (Effects|SpawnEmitteratLocation "/Game/MilitaryWeapDark/FX/P_Grenade_Explosion_01.P_Grenade_Explosion_01" (.location (Transformation|GetActorTransform _asbp_turret)) (.rotation (Transformation|GetActorTransform _asbp_turret)) (.scale (Transformation|GetActorTransform _asbp_turret)))
  (Utilities|IsValid self
    (:Is%20Valid
      (Actor|DestroyActor)
      (Class|LegacyCameraShake|StartLegacyCameraShake (Game|GetPlayerCameraManager 0) "/Game/Blueprints/BP_CameraShake.BP_CameraShake_C" 0.85 "CameraLocal" "0, 0, 0")
      (Actor|DestroyActor _asbp_turret))))

(event Custom|Lock%20on
  (bind _projectile (Variables|Default|GetProjectile))
  ;[0 1 1] Find Target
  (bind _homing_target (CallFunction|FindHomingTarget))
  (Variables|/Script/Engine.ProjectileMovementComponent|SetHomingTargetComponent _projectile _homing_target)
  (Variables|/Script/Engine.ProjectileMovementComponent|SetbIsHomingProjectile _projectile true))

(event EventBeginPlay
  ;[1 0 1] Lock On To Target
  (Utilities|FlowControl|Delay (Variables|Default|GetLock%20On%20Time))
  (CallFunction|Lockon :!label _label)
  (Utilities|FlowControl|Delay 0.1)
  (goto _label))

(fn ConstructionScript)

(fn FindHomingTarget
  (bind _outactors (Actor|GetAllActorsOfClass "/Game/_Game/Blueprints/Actors/BP_Turret.BP_Turret_C"))
  (for _array_element _outactors
    (Utilities|IsValid _array_element
      (:Is%20Valid
        (Variables|Default|SetHoming%20Target _array_element)
        (if (< (Math|Vector|VectorLength (- (Transformation|GetActorLocation _array_element) (Transformation|GetActorLocation))) (Variables|Default|GetCloset%20Distance))
          (Variables|Default|SetCloset%20Distance (Math|Vector|VectorLength (- (Transformation|GetActorLocation _array_element) (Transformation|GetActorLocation))))))))
  (Utilities|IsValid (Actor|GetComponentbyClass (Variables|Default|GetHoming%20Target) "/Script/Engine.SceneComponent")
    (:Is%20Valid
      (return (Actor|GetComponentbyClass (Variables|Default|GetHoming%20Target) "/Script/Engine.SceneComponent")))))