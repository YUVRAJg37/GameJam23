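; World-gen actor that gives its static mesh a random look, picking a mesh from the Buildings array and a random rotation.
; All work happens in the Construction Script, using unseeded random, so the result re-rolls whenever construction reruns.
; A helper rolls each rotation axis independently between zero and MaxBuildingRandomRotation, applied as world rotation at the mesh's current location.
; An empty array skips both steps, and the event graph is unused.
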(event EventBeginPlay)

(event Collision|EventActorBeginOverlap
  (params (OtherActor :type Actor%20Object%20Reference)))

(event EventTick
  (params (DeltaSeconds :type Float%20%28single-precision%29)))

(fn ConstructionScript
  (bind _buildings (Variables|Default|GetBuildings))
  (bind _staticmesh (Variables|Default|GetStaticMesh))
  (if (Utilities|Array|IsNotEmpty _buildings)
    (Components|StaticMesh|SetStaticMesh _staticmesh (Utilities|Array|Get(acopy) _buildings (Math|Random|RandomInteger (Utilities|Array|Length _buildings))))
    (Transformation|SetWorldTransform (Variables|Default|GetStaticMesh) (Math|Transform|MakeTransform (Transformation|GetWorldLocation _staticmesh) (CallFunction|GetRandomRotationinRange "0, 0, 0" (Variables|Default|GetMaxBuildingRandomRotation)) "1.000000,1.000000,1.000000") false false)))

(fn GetRandomRotationinRange
  (params (MinRotation :type Rotator) (MaxRotation :type Rotator))
  (bind (_roll _pitch _yaw) (Math|Rotator|BreakRotator MaxRotation))
  (bind (_roll_2 _pitch_2 _yaw_2) (Math|Rotator|BreakRotator MinRotation))
  (return (Math|Rotator|MakeRotator (Math|Random|RandomFloatinRange _roll_2 _roll) (Math|Random|RandomFloatinRange _pitch_2 _pitch) (Math|Random|RandomFloatinRange _yaw_2 _yaw))))