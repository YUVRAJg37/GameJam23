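; BP_ObstacleGen is a world-generation segment that fills itself with obstacles for the aircraft to fly through.
; On BeginPlay it randomly passes either an arch mesh or a ball mesh to GenerateInstance, with BP_Turret as the actor class.
; When BP_Aircraft overlaps EndTrigger, it asks BP_PlaneGameMode to add another BP_ObstacleGen, then destroys itself after a short delay.
; GetAttachTransform exposes the AttachPoint world transform.
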(event OnComponentBeginOverlap(EndTrigger)
  (params (OverlappedComponent :type Primitive%20Component%20Object%20Reference) (OtherActor :type Actor%20Object%20Reference) (OtherComp :type Primitive%20Component%20Object%20Reference) (OtherBodyIndex :type Integer) (bFromSweep :type Boolean) (SweepResult :type Hit%20Result%20Structure%20%28by%20ref%29))
  (Utilities|Casting|CastToBP_Aircraft OtherActor)
  (bind _asbp_plane_game_mode (Utilities|Casting|CastToBP_PlaneGameMode (Game|GetGameMode)))
  (Default|AddSides _asbp_plane_game_mode false "BP_ObstacleGen_C")
  (Utilities|FlowControl|Delay 2.0)
  (Actor|DestroyActor))

(event EventBeginPlay
  (if (Math|Random|RandomBool)
    (CallFunction|GenerateInstance "/Game/_Game/Assets_Yuvi/Buildings/Arch.Arch" 2 true false "0, 0, 0" "0, 0, 0" 0.01 false "/Game/_Game/Blueprints/Actors/BP_Turret.BP_Turret_C")
    (else
      (CallFunction|GenerateInstance "/Engine/VREditor/BasicMeshes/SM_Ball_01.SM_Ball_01" 1 true false "0, 0, 0" "0, 0, 0" 0.2 true "/Game/_Game/Blueprints/Actors/BP_Turret.BP_Turret_C"))))

(event Collision|EventActorBeginOverlap
  (params (OtherActor :type Actor%20Object%20Reference)))

(fn ConstructionScript
  (|CallParentFunction))

(fn GetAttachTransform
  (return (Transformation|GetWorldTransform (Variables|Default|GetAttachPoint))))