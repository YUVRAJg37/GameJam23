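; BP_RandomWorldGen is a world-generation actor that scatters mesh instances or spawned actors at random points inside its Box bounds.
; GenerateInstance resets the InstancedStaticMesh to world origin, clears it, then rolls a spawn chance for each of a fixed or randomized count.
; Meshes can receive random per-axis scale, while actors receive random yaw.
; Nothing here calls GenerateInstance; events, construction script and GetAttachTransform are empty.
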(event EventBeginPlay)

(event Collision|EventActorBeginOverlap
  (params (OtherActor :type Actor%20Object%20Reference)))

(event EventTick
  (params (DeltaSeconds :type Float%20%28single-precision%29)))

(fn ConstructionScript)

(fn GetAttachTransform
  (return ""))

(fn GenerateInstance
  (params (Mesh :type Static%20Mesh%20Object%20Reference) (Amount :type Integer) (Randomize%20Amount :type Boolean) (Randomize%20Scale :type Boolean) (Min%20Scale :type Vector) (Max%20Scale :type Vector) (Spawn%20Chance :type Float%20%28double-precision%29) (Actor? :type Boolean) (ActorClass :type Actor%20Class%20Reference))
  (bind _instancedstaticmesh (Variables|Default|GetInstancedStaticMesh))
  (bind _box (Variables|Default|GetBox))
  (bind (_x _y _z) (Math|Vector|BreakVector Min%20Scale))
  (bind (_origin _boxextent) (Collision|GetComponentBounds _box))
  (bind (_x_2 _y_2 _z_2) (Math|Vector|BreakVector Max%20Scale))
  (bind _returnvalue (Math|Random|RandomPointinBoundingBox _origin _boxextent))
  (if true
    (Transformation|SetWorldLocation _instancedstaticmesh "0, 0, 0" false false)
    (Components|InstancedStaticMesh|ClearInstances _instancedstaticmesh)
    (if Actor?
      _
      (else
        (Components|StaticMesh|SetStaticMesh (Variables|Default|GetInstancedStaticMesh) Mesh)))
    (if Randomize%20Amount
      (LocalVariables|SetMaxSpawnAmount (Math|Random|RandomIntegerinRange 0 Amount))
      (else
        (LocalVariables|SetMaxSpawnAmount Amount)))
    (for _index (range 0 (LocalVariables|GetMaxSpawnAmount))
      (if (< (Math|Random|RandomFloatinRange 0.0 1e+02) (* Spawn%20Chance 1e+02))
        (if Actor?
          (Game|SpawnActorfromClass ActorClass (Math|Transform|MakeTransform _returnvalue (Math|Rotator|MakeRotator 0.0 0.0 (Math|Random|RandomFloatinRange 0.0 3.6e+02)) "1.000000,1.000000,1.000000") "Undefined" 0 0)
          (elif Randomize%20Scale
            (Components|InstancedStaticMesh|AddInstance (Variables|Default|GetInstancedStaticMesh) (Math|Transform|MakeTransform _returnvalue "0, 0, 0" (Math|Vector|MakeVector (Math|Random|RandomFloatinRange _x _x_2) (Math|Random|RandomFloatinRange _y _y_2) (Math|Random|RandomFloatinRange _z _z_2))) false)
            (else
              (Components|InstancedStaticMesh|AddInstance (Variables|Default|GetInstancedStaticMesh) (Math|Transform|MakeTransform _returnvalue "0, 0, 0" "1.000000,1.000000,1.000000") false))))))))