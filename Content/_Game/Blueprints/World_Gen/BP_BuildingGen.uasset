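; BP_BuildingGen is a world-generation tile that scatters randomly scaled cube buildings as scenery for the plane game.
; On BeginPlay it calls GenerateInstance with randomized amount and scale, stretching the cubes tallest on Z.
; When BP_Aircraft overlaps EndTrigger, it has BP_PlaneGameMode add new BP_BuildingGen tiles on two sides, then destroys itself after a short delay.
; GetAttachTransform exposes the AttachPoint world transform.
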(event OnComponentBeginOverlap(EndTrigger)
  (params (OverlappedComponent :type Primitive%20Component%20Object%20Reference) (OtherActor :type Actor%20Object%20Reference) (OtherComp :type Primitive%20Component%20Object%20Reference) (OtherBodyIndex :type Integer) (bFromSweep :type Boolean) (SweepResult :type Hit%20Result%20Structure%20%28by%20ref%29))
  (Utilities|Casting|CastToBP_Aircraft OtherActor)
  (bind _asbp_plane_game_mode (Utilities|Casting|CastToBP_PlaneGameMode (Game|GetGameMode)))
  (Default|AddSides _asbp_plane_game_mode true "BP_BuildingGen_C")
  (Utilities|FlowControl|Delay 2.0)
  (Actor|DestroyActor))

(event EventBeginPlay
  (CallFunction|GenerateInstance "/Engine/VREditor/BasicMeshes/SM_Cube_01.SM_Cube_01" 20 true true "1.000000,1.000000,2.000000" "5.000000,5.000000,20.000000" 1.0 false))

(event Collision|EventActorBeginOverlap
  (params (OtherActor :type Actor%20Object%20Reference)))

(event EventTick
  (params (DeltaSeconds :type Float%20%28single-precision%29)))

(fn ConstructionScript)

(fn GetAttachTransform
  (return (Transformation|GetWorldTransform (Variables|Default|GetAttachPoint))))