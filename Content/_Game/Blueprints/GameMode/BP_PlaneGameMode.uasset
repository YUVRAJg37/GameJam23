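; BP_PlaneGameMode is a game mode that lays out the world when play begins.
; It spawns ten rounds of building generators on left and right tracks, plus an obstacle generator on a single track.
; Each track chains pieces: AddBuilding spawns at that track's next spawn transform, then overwrites it by reference with the new BP_RandomWorldGen actor's attach transform.
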(event EventBeginPlay
  (for _index (range 0 9)
    (CallFunction|AddSides true "/Game/_Game/Blueprints/World_Gen/BP_BuildingGen.BP_BuildingGen_C")
    (CallFunction|AddSides false "/Game/_Game/Blueprints/World_Gen/BP_ObstacleGen.BP_ObstacleGen_C")))

(fn ConstructionScript)

(fn AddBuilding
  (params (Actor%20to%20Spawn :type Actor%20Class%20Reference) (Transform :type Transform%20%28by%20ref%29))
  (bind _returnvalue (Game|SpawnActorfromClass Actor%20to%20Spawn Transform "Undefined" 0 0))
  (bind _asbp_random_world_gen (Utilities|Casting|CastToBP_RandomWorldGen _returnvalue))
  (|SetBy-RefVar Transform (Default|GetAttachTransform _asbp_random_world_gen)))

(fn AddSides
  (params (Two%20Sides :type Boolean) (Actor%20To%20Spawn :type Actor%20Class%20Reference))
  (if Two%20Sides
    (CallFunction|AddBuilding Actor%20To%20Spawn (Variables|Default|GetNextSpawnPointLeft))
    (CallFunction|AddBuilding Actor%20To%20Spawn (Variables|Default|GetNextSpawnPointRight))
    (else
      (CallFunction|AddBuilding Actor%20To%20Spawn (Variables|Default|GetNextSpawnPoint)))))