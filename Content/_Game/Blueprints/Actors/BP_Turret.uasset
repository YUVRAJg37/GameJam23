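; BP_Turret is a turret actor whose gun tracks the BP_Aircraft in the level.
; On BeginPlay it finds the aircraft if unset, then spawns and attaches a BP_ProjectileSpawner at each of its Left and Right mount points.
; Each Tick it smoothly rotates the gun with RInterpTo, using a look-at rotation computed from plane to gun, so the gun's +X axis points away from the aircraft.
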(event EventBeginPlay
  (Utilities|IsValid (Variables|Default|GetBP_Plane)
    (:Is%20Valid
      _)
    (:Is%20Not%20Valid
      (bind _returnvalue (Actor|GetActorOfClass "/Game/Blueprints/BP_Aircraft.BP_Aircraft_C"))
      (Variables|Default|SetBP_Plane _returnvalue)))
  (bind _returnvalue_2 (Game|SpawnActorfromClass "/Game/_Game/Blueprints/Actors/Porjectile/BP_ProjectileSpawner.BP_ProjectileSpawner_C" (Transformation|GetWorldTransform (Variables|Default|GetLeft)) "Undefined" 0 0))
  (Transformation|AttachComponentToComponent _returnvalue_2 (Variables|Default|GetLeft) "None" "KeepWorld" "KeepWorld" "KeepWorld" false)
  (bind _returnvalue_3 (Game|SpawnActorfromClass "/Game/_Game/Blueprints/Actors/Porjectile/BP_ProjectileSpawner.BP_ProjectileSpawner_C" (Transformation|GetWorldTransform (Variables|Default|GetRight)) "Undefined" 0 0))
  (Transformation|AttachComponentToComponent _returnvalue_3 (Variables|Default|GetRight) "None" "KeepWorld" "KeepWorld" "KeepWorld" false))

(event EventTick
  (params (DeltaSeconds :type Float%20%28single-precision%29))
  (Utilities|IsValid (Variables|Default|GetBP_Plane)
    (:Is%20Valid
      (Transformation|SetWorldRotation (Variables|Default|GetGun) (Math|Interpolation|RInterpTo (Transformation|GetWorldRotation (Variables|Default|GetGun)) (CallFunction|GetLookatRotationforPlane) DeltaSeconds 1.2) false false))))

(fn ConstructionScript)

(fn GetLookatRotationforPlane
  (return (Math|Rotator|FindLookatRotation (Transformation|GetActorLocation (Variables|Default|GetBP_Plane)) (Transformation|GetWorldLocation (Variables|Default|GetGun)))))